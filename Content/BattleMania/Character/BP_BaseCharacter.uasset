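; BP_BaseCharacter is a character Blueprint that sets up the player's on-screen UI and minimap in BattleMania.
; On BeginPlay it shows a player info widget for the locally controlled character, then creates the player HUD without that locality check.
; The HUD's minimap widget is cached and registered with MiniMapGameState.
; Add and Subtract keys step the minimap's Zoom value down and up.
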(event EventBeginPlay
  (Utilities|FlowControl|Sequence
    (:then_0
      (if (Pawn|IsLocallyControlled)
        (bind _returnvalue (UserInterface|CreateWidget "/Game/BattleMania/Blueprint/WBP_PlayerInfo.WBP_PlayerInfo_C"))
        (bind _output_get (Variables|Default|SetPlayerInfoWidget _returnvalue))
        (UserInterface|Viewport|AddtoViewport _output_get 0)))
    (:then_1
      ;[1 1 1] MiniMap
      (bind _returnvalue_2 (UserInterface|CreateWidget "/Game/WBP_PlayerHUD.WBP_PlayerHUD_C"))
      (bind _output_get_2 (Variables|Default|SetPlayerHUD _returnvalue_2))
      (UserInterface|Viewport|AddtoViewport _output_get_2 0)
      (Variables|Default|SetMiniMapWidget (Variables|/Game/WBP_PlayerHUD.WBP_PlayerHUD_C|GetWBP_MiniMapWidget _output_get_2)))
    (:then_2
      (bind _asmini_map_game_state (Utilities|Casting|CastToMiniMapGameState (Game|GetGameState)))
      (Class|MiniMapGameState|RegisterMap _asmini_map_game_state (Variables|Default|GetMiniMapWidget)))))

(event Input|KeyboardEvents|Add
  (params (Key :type Key%20Structure))
  (bind _minimapwidget (Variables|Default|GetMiniMapWidget))
  ;[1 1 1] Map Zoom
  (:Pressed
    (Variables|/Script/MiniMapModule.MapWidget|SetZoom _minimapwidget (- (Variables|/Script/MiniMapModule.MapWidget|GetZoom _minimapwidget) 0.1))))

(event Input|KeyboardEvents|Subtract
  (params (Key :type Key%20Structure))
  (bind _minimapwidget (Variables|Default|GetMiniMapWidget))
  ;[1 1 1] Map Zoom
  (:Pressed
    (Variables|/Script/MiniMapModule.MapWidget|SetZoom _minimapwidget (+ (Variables|/Script/MiniMapModule.MapWidget|GetZoom _minimapwidget) 0.1))))

(fn ConstructionScript)